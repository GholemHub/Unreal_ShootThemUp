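; BP_TestBlock is a test block for block placement that starts as a preview and becomes solid when placed.
; On BeginPlay it stores the cube's original material, applies the BlockPreview material and disables collision.
; The Placed event restores the stored material and enables query and physics collision.
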(event Custom|Placed
  (Rendering|Material|SetMaterial (Variables|Default|GetCube) 0 (Variables|Default|GetDefaultMaterial))
  (Collision|SetCollisionEnabled (Variables|Default|GetCube) "QueryAndPhysics"))

(event EventBeginPlay
  (bind _cube (Variables|Default|GetCube))
  (Variables|Default|SetDefaultMaterial (Rendering|Material|GetMaterial _cube 0))
  (Rendering|Material|SetMaterial _cube 0 "/Game/BlockPlacement/Materials/BlockPreview.BlockPreview")
  (Collision|SetCollisionEnabled (Variables|Default|GetCube) "NoCollision"))

(event Collision|EventActorBeginOverlap
  (params (OtherActor :type Actor%20Object%20Reference)))

(fn ConstructionScript
  (|CallParentFunction))